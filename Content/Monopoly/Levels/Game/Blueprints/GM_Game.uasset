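; Game mode for a multiplayer Monopoly match that handles player setup, game start and turn order.
; Each joining controller possesses a spawned pawn; once MaxPlayers have joined, it initializes client UI and picks a random starting player.
; CycleTurns resets turn state, triggers auction messages on the game state and advances past bankrupt players, incrementing the turn count on returning to the starting player.
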(event Custom|StartGame
  (bind _asgs_game (Utilities|GetGameState))
  ;[1 1 1] Setup
  (for _array_element (Variables|References|GetPlayerControllers)
    (Default|InitUICLIENT _array_element))
  (bind _returnvalue (Class|GameModeBase|GetNumPlayers))
  (Variables|Default|SetActivePlayer (Math|Random|RandomInteger _returnvalue))
  (Default|PickStartingPlayer _asgs_game (Variables|/Script/Engine.PlayerState|GetPlayerId (Utilities|GetActivePlayerState)))
  (CallFunction|SetActivePlayerTurn true)
  (Variables|/Game/Monopoly/Levels/Game/Blueprints/GS_Game.GS_Game_C|SetPlaying _asgs_game true))

(event EventCycleTurns
  (bind _asgs_game (Utilities|GetGameState))
  ;[1 1 1] Turn Cycling
  (Default|ResetTurnSpecific _asgs_game)
  (Class|GSIGame|AuctionifNotBought(Message) _asgs_game)
  (Class|GSIGame|CheckAuctions(Message) _asgs_game)
  (CallFunction|SetActivePlayerTurn false)
  (CallFunction|SwapActivePlayer :!label _label)
  (if (Variables|/Game/Monopoly/Levels/Game/Blueprints/PS_Game.PS_Game_C|GetbBankrupt (Utilities|GetActivePlayerState))
    (goto _label)
    (else
      (CallFunction|SetActivePlayerTurn true))))

(event EventHandleStartingNewPlayer
  (params (NewPlayer :type Player%20Controller%20Object%20Reference))
  (bind _playercontrollers (Variables|References|GetPlayerControllers))
  (bind _returnvalue (Utilities|Array|Length _playercontrollers))
  ;[1 1 1] Setup
  (bind _aspc_game (Utilities|Casting|CastToPC_Game NewPlayer))
  (Utilities|Array|AddUnique _playercontrollers _aspc_game)
  (bind _returnvalue_2 (Game|SpawnActorfromClass "/Game/Monopoly/Levels/Game/Blueprints/PN_Game.PN_Game_C" (Math|Transform|MakeTransform "0, 0, 0") "AlwaysSpawn" 0 0))
  (Pawn|Possess _aspc_game _returnvalue_2)
  (if (== _returnvalue (Variables|Default|GetMaxPlayers))
    (Variables|/Game/Monopoly/Levels/Game/Blueprints/GS_Game.GS_Game_C|SetNumPlayers (Utilities|GetGameState) _returnvalue)
    (CallFunction|StartGame)))

(fn ConstructionScript)

(fn SetActivePlayerTurn
  (params (MyTurn :type Boolean))
  (bind _aspc_game (Utilities|GetActivePlayerController))
  (bind _aspc_game_2 (Utilities|GetActivePlayerController))
  (if MyTurn
    (Default|StartTurnCLIENT _aspc_game_2)
    (Class|PSIGame|SetStatus(Message) (Variables|/Script/Engine.Controller|GetPlayerState _aspc_game_2) "NewEnumerator1")
    (else
      (Default|EndTurnCLIENT _aspc_game)
      (Class|PSIGame|SetStatus(Message) (Variables|/Script/Engine.Controller|GetPlayerState _aspc_game) "NewEnumerator0"))))

(fn SwapActivePlayer
  (bind _asgs_game (Utilities|GetGameState))
  (Variables|Default|SetActivePlayer (Math|Integer|%(Integer) (+ (Variables|Default|GetActivePlayer) 1) (Variables|/Game/Monopoly/Levels/Game/Blueprints/GS_Game.GS_Game_C|GetNumPlayers _asgs_game)))
  (Variables|/Game/Monopoly/Levels/Game/Blueprints/GS_Game.GS_Game_C|SetActivePlayerId (Utilities|GetGameState) (Variables|/Script/Engine.PlayerState|GetPlayerId (Utilities|GetActivePlayerState)))
  (if (== (Variables|/Script/Engine.PlayerState|GetPlayerId (Utilities|GetActivePlayerState)) (Variables|/Game/Monopoly/Levels/Game/Blueprints/GS_Game.GS_Game_C|GetStartingPlayer _asgs_game))
    (Math|Integer|IncrementInt (Variables|/Game/Monopoly/Levels/Game/Blueprints/GS_Game.GS_Game_C|GetTurn (Utilities|GetGameState)))))