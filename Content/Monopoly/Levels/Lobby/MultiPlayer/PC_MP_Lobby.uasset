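; Player controller for the Monopoly multiplayer lobby, linking each player's lobby UI to the server.
; On BeginPlay a looping timer polls until the GameState's player array is populated, then submits player info as not ready and creates the lobby widget.
; Server events copy the GameInstance's online info and ready flag into the PlayerState and have the lobby GameMode check whether play can start.
; Client events update the message, refresh other players or remove the UI.
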(event Custom|ClearUI%20CLIENT
  (Widget|RemovefromParent (Variables|Default|GetLobbyMainRef)))

(event Custom|SRV%20-%20CheckReady
  (Default|CheckCanStart (.AsGM%20MP%20Lobby (Utilities|Casting|CastToGM_MP_Lobby (Game|GetGameMode)))))

(event Custom|RefreshOthers%20CLIENT
  (bind _lobbymainref (Variables|Default|GetLobbyMainRef))
  (Utilities|IsValid _lobbymainref
    (:Is%20Valid
      (Default|RefreshOthers _lobbymainref))))

(event Custom|SetPSInfos%20CLIENT
  (params (bIsReady :type Boolean))
  (CallFunction|SRV-SetPSInfos (Variables|/Game/Monopoly/Levels/AllLevels/MonopolyGameInstance.MonopolyGameInstance_C|GetOnlineInfos (Utilities|GetGI)) bIsReady)
  (CallFunction|SRV-CheckReady))

(event Custom|GSIsHere
  (if (Math|Conversions|ToBoolean(Integer) (Utilities|Array|Length (Variables|/Script/Engine.GameStateBase|GetPlayerArray (Game|GetGameState))))
    (Utilities|Time|ClearandInvalidateTimerbyHandle (stale Custom|Init%20CLIENT _returnvalue))
    (CallFunction|SetPSInfosCLIENT false)
    (CallFunction|SetUI)))

(event Custom|Init%20CLIENT
  (bind _returnvalue (Utilities|Time|SetTimerbyEvent (delegate Custom|GSIsHere) 0.1 true)))

(event Custom|StartMessage%20CLIENT
  (params (InText :type Text))
  (Default|Changetext (Variables|Default|GetLobbyMainRef) InText))

(event Custom|SRV%20-%20SetPSInfos
  (params (PlayerInfos :type ST%20Player%20Data%20Structure) (bIsReady :type Boolean))
  (bind _asps_lobby (Utilities|GetPS))
  (Variables|/Game/Monopoly/Levels/Lobby/MultiPlayer/PS_MP_Lobby.PS_MP_Lobby_C|SetPlayerInfos _asps_lobby PlayerInfos)
  (Variables|/Game/Monopoly/Levels/Lobby/MultiPlayer/PS_MP_Lobby.PS_MP_Lobby_C|SetbIsReady _asps_lobby bIsReady))

(event EventBeginPlay
  (CallFunction|InitCLIENT))

(fn ConstructionScript)

(fn SetUI
  (bind _returnvalue (UserInterface|CreateWidget "/Game/Monopoly/Levels/Lobby/MultiPlayer/UI_MP_LobbyMain.UI_MP_LobbyMain_C"))
  (Variables|Default|SetLobbyMainRef _returnvalue)
  (UserInterface|Viewport|AddtoViewport _returnvalue 0))