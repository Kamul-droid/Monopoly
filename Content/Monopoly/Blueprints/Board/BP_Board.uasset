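; Monopoly board actor that holds references to every BP_BoardSquare and answers lookups on them.
; Initialize gathers the squares from the level once, initializing each and storing it at the array index given by its N.
; GetSquare returns a square by index with a validity flag.
; GetNextOfType searches forward from a given index, wrapping by modulo and checking the starting square last, to find the next square of a type.
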(event EventBeginPlay)

(event Collision|EventActorBeginOverlap
  (params (OtherActor :type Actor%20Object%20Reference)))

(event EventTick
  (params (DeltaSeconds :type Float%20%28single-precision%29)))

(fn ConstructionScript)

(fn Initialize
  (Setup|SetSquaresRefs))

(fn SetSquaresRefs
  (if (== (Utilities|Array|Length (Variables|References|GetBoardSquaresRef)) 0)
    (bind _outactors (Actor|GetAllActorsOfClass "/Game/Monopoly/Blueprints/Board/BP_BoardSquare.BP_BoardSquare_C"))
    (for _array_element _outactors
      (Default|Initialize _array_element)
      (Utilities|Array|SetArrayElem (Variables|References|GetBoardSquaresRef) (Variables|/Game/Monopoly/Blueprints/Board/BP_BoardSquare.BP_BoardSquare_C|GetN _array_element) _array_element true))))

(fn GetSquare
  (params (SquareIndex :type Integer))
  (bind _boardsquaresref (Variables|References|GetBoardSquaresRef))
  (return (Utilities|Array|Get(acopy) _boardsquaresref SquareIndex) (Utilities|Array|IsValidIndex _boardsquaresref SquareIndex)))

(fn GetNextOfType
  (params (Type :type EN_SquareType%20Enum :default "NewEnumerator0") (From :type Integer))
  (bind _boardsquaresref (Variables|References|GetBoardSquaresRef))
  (bind _returnvalue (Utilities|Array|Length _boardsquaresref))
  ;[1 1 1 1 12] Local variable for cleaner management
  (LocalVariables|SetTypeToCheck Type)
  ;[1 1 1 1 12] Goes from x+1 to x
  (for _index (range (+ From 1) (+ From _returnvalue))
    (if (Utilities|Enum|Equal(Enum) (LocalVariables|GetTypeToCheck) (.SquareType (Utilities|Struct|BreakST_SquareData (Variables|/Game/Monopoly/Blueprints/Board/BP_BoardSquare.BP_BoardSquare_C|GetGridData (Utilities|Array|Get(acopy) (Variables|References|GetBoardSquaresRef) (Math|Integer|%(Integer) _index _returnvalue))))))
      (return (Math|Integer|%(Integer) _index _returnvalue)))))