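; Player controller for the Monopoly match, acting as each player's link between the game UI and the server.
; On client init it polls until the game state, board and full player list exist, then creates and populates the game UI.
; SRV-prefixed events forward dice, property, trade, auction, jail, debug and chat actions to GS_Game, while turn ending goes to the game mode.
; It also tracks whose turn it is and appends chat messages with smart auto-scroll.
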(event Custom|SRV%20-%20ThrowDice
  (Class|GSIGame|ThrowDice(Message) (Game|GetGameState)))

(event Custom|StartTurn%20CLIENT
  (CallFunction|SetMyTurn true))

(event Custom|SRV%20-%20BuyProperty
  (Class|GSIGame|BuyProperty(Message) (Game|GetGameState)))

(event Custom|SRV%20-%20AddTrade
  (params (Trade :type ST%20Trade%20Structure))
  (Class|GSIGame|AddTrade(Message) (Game|GetGameState) Trade))

(event Custom|SRV%20-%20RejectTrade
  (params (Trade :type ST%20Trade%20Structure))
  (Class|GSIGame|RemoveTrade(Message) (Game|GetGameState) Trade))

(event Custom|SRV%20-%20AcceptTrade
  (params (Trade :type ST%20Trade%20Structure))
  (Class|GSIGame|ProcessTrade(Message) (Game|GetGameState) Trade))

(event Custom|SRV%20-%20Bid
  (params (Square :type BP%20Square%20Object%20Reference) (Bid :type Integer))
  (Class|GSIGame|Bid(Message) (Game|GetGameState) Square Bid (Variables|/Script/Engine.PlayerState|GetPlayerId (Variables|GetPlayerState))))

(event Custom|PayDebt
  (params (Debt :type ST%20Debt%20Structure))
  (Class|GSIGame|PayDebt(Message) (Game|GetGameState) Debt))

(event Custom|SRV%20-%20DeclareBankruptcy
  (Class|GSIGame|DeclareBankruptcy(Message) (Game|GetGameState) (Variables|/Script/Engine.PlayerState|GetPlayerId (Variables|GetPlayerState))))

(event Custom|SRV%20-%20Unmortagage
  (params (Square :type BP%20Square%20Object%20Reference))
  (Class|GSIGame|Unmortgage(Message) (Game|GetGameState) (Variables|/Script/Engine.PlayerState|GetPlayerId (Variables|GetPlayerState)) Square))

(event Custom|SRV%20-%20BuyHouse
  (params (Square :type BP%20Square%20Object%20Reference))
  (Class|GSIGame|BuyHouse(Message) (Game|GetGameState) (Variables|/Script/Engine.PlayerState|GetPlayerId (Variables|GetPlayerState)) Square))

(event Custom|SRV%20-%20SendMessage
  (params (Message :type String))
  (Default|SendMessage (.AsGS%20Game (Utilities|Casting|CastToGS_Game (Game|GetGameState))) (Utilities|String|Append (Variables|/Game/Monopoly/Levels/Game/Blueprints/PS_Game.PS_Game_C|GetName (.AsPS%20Game (Utilities|Casting|CastToPS_Game (Variables|GetPlayerState)))) " : " Message)))

(event Custom|InitUI%20CLIENT
  (bind _returnvalue (Utilities|Time|SetTimerbyEvent (delegate Custom|IsGamestateHere) 0.1 true)))

(event Custom|SRV%20-%20SellHouse
  (params (Square :type BP%20Square%20Object%20Reference))
  (Class|GSIGame|SellHouse(Message) (Game|GetGameState) (Variables|/Script/Engine.PlayerState|GetPlayerId (Variables|GetPlayerState)) Square))

(event Custom|SRV%20-%20Mortgage
  (params (Square :type BP%20Square%20Object%20Reference))
  (Class|GSIGame|Mortgage(Message) (Game|GetGameState) (Variables|/Script/Engine.PlayerState|GetPlayerId (Variables|GetPlayerState)) Square))

(event Custom|GetMessage
  (params (Message :type String))
  (bind _uigameref (Variables|Default|GetUIGameRef))
  (bind _ui_chatbox (Variables|/Game/Monopoly/Levels/Game/UI/UI_Game.UI_Game_C|GetUI_ChatBox _uigameref))
  (bind _chatcontainer (Variables|/Game/Monopoly/Levels/Game/UI/UI_ChatBox.UI_ChatBox_C|GetChatContainer _ui_chatbox))
  (Utilities|IsValid (Variables|Default|GetUIGameRef)
    (:Is%20Valid
      (bind _returnvalue (UserInterface|CreateWidget "/Game/Monopoly/Levels/Game/UI/UI_ChatBoxMessage.UI_ChatBoxMessage_C" 0 Message))
      (if (== (- (Class|ScrollBox|GetScrollOffsetOfEnd _chatcontainer) (Class|ScrollBox|GetScrollOffset _chatcontainer)) 0.0)
        (Widget|Panel|AddChild _chatcontainer _returnvalue)
        (Class|ScrollBox|ScrolltoEnd _chatcontainer)
        (else
          (Widget|Panel|AddChild _chatcontainer _returnvalue))))))

(event Custom|SRV%20-%20OutOfJail
  (params (UseCard :type Boolean))
  (bind _returnvalue (Game|GetGameState))
  (if UseCard
    (Class|GSIGame|UseJailCard(Message) _returnvalue)
    (else
      (Class|GSIGame|PayJailFine(Message) _returnvalue))))

(event Custom|EndTurn%20CLIENT
  (CallFunction|SetMyTurn false))

(event Custom|SRV%20-%20EndTurn
  (Class|GMIGame|CycleTurns(Message) (Game|GetGameMode)))

(event Custom|SRV%20-%20DoCommunity
  (params (Community :type EN_Community%20Enum :default "NewEnumerator0"))
  (Default|DoCommunityCommand (.AsGS%20Game (Utilities|Casting|CastToGS_Game (Game|GetGameState))) Community))

(event Custom|SRV%20-%20DoChance
  (params (Chance :type EN_Chance%20Enum :default "NewEnumerator0"))
  (Default|DoChanceCommand (.AsGS%20Game (Utilities|Casting|CastToGS_Game (Game|GetGameState))) Chance))

(event Custom|IsGamestateHere
  (bind _returnvalue (Game|GetGameState))
  (bind _uigameref (Variables|Default|GetUIGameRef))
  (bind _asgs_game (Utilities|Casting|CastToGS_Game _returnvalue))
  (Utilities|IsValid _returnvalue
    (:Is%20Valid
      (Utilities|IsValid (Variables|/Game/Monopoly/Levels/Game/Blueprints/GS_Game.GS_Game_C|GetBoard _asgs_game)
        (:Is%20Valid
          (if (== (Utilities|Array|Length (Variables|/Script/Engine.GameStateBase|GetPlayerArray _returnvalue)) (Variables|/Game/Monopoly/Levels/Game/Blueprints/GS_Game.GS_Game_C|GetNumPlayers _asgs_game))
            (Utilities|Time|ClearandInvalidateTimerbyHandle (stale Custom|InitUI%20CLIENT _returnvalue))
            (CallFunction|SetUIRef)
            (UserInterface|Viewport|AddtoViewport _uigameref 0)
            (Default|PopulatePlayers _uigameref)))))))

(event Custom|SRV%20-%20ResetMoney
  (Class|PSIGame|ResetMoney(Message) (Variables|GetPlayerState)))

(event Custom|SRV%20-%20DoctoredDice
  (params (Value :type Integer) (Double :type Boolean))
  (Class|GSIGame|DoctoredDice(Message) (Game|GetGameState) Value Double))

(fn ConstructionScript)

(fn SetMyTurn
  (params (MyTurn :type Boolean))
  (Variables|Default|SetMyTurn MyTurn))

(fn SetUIRef
  (bind _returnvalue (UserInterface|CreateWidget "/Game/Monopoly/Levels/Game/UI/UI_Game.UI_Game_C" self))
  (Variables|Default|SetUIGameRef _returnvalue))

(fn ShowPlayerUI
  (bind _uigameref (Variables|Default|GetUIGameRef))
  (UserInterface|Viewport|AddtoViewport _uigameref 0)
  (Default|PopulatePlayers _uigameref))

(fn HidePlayerUI
  (Widget|RemovefromParent (Variables|Default|GetUIGameRef)))