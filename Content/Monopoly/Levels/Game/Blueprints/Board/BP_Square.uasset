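; Monopoly board square actor that tracks its owner, houses and hotel, and reports clicks to the game state's board for selection.
; It answers rule checks for buying, mortgaging and building, using board queries for monopolies and house counts in the color group.
; Rent depends on type: property uses the board's price table, railways double per extra one owned, utilities multiply the dice roll, and a BiggerFine flag raises the latter two.
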(event OnClicked(Square)
  (params (TouchedComponent :type Primitive%20Component%20Object%20Reference) (ButtonPressed :type Key%20Structure))
  (Default|SelectSquare (Variables|/Game/Monopoly/Levels/Game/Blueprints/GS_Game.GS_Game_C|GetBoard (.AsGS%20Game (Utilities|Casting|CastToGS_Game (Game|GetGameState)))) (Variables|Setup|GetN)))

(event EventBeginPlay)

(event Collision|EventActorBeginOverlap
  (params (OtherActor :type Actor%20Object%20Reference)))

(event EventTick
  (params (DeltaSeconds :type Float%20%28single-precision%29)))

(fn ConstructionScript)

(fn OwnershipStatus
  (params (PlayerIndex :type Integer))
  (bind _playerowner (Variables|Gameplay|GetPlayerOwner))
  (return (!= _playerowner -1) (== PlayerIndex _playerowner) _playerowner))

(fn SetMarkerVisible
  (params (Visible :type Boolean))
  (Rendering|SetVisibility (Variables|Default|GetMarker) Visible false))

(fn CanMortgage
  (params (PlayerIndex :type Integer))
  (return (and (.IsOwner (GamePlay|OwnershipStatus PlayerIndex)) (== (.Max (Default|MinMaxHousesinColor (Utilities|GetBoard) (Utilities|Struct|BreakST_SquareData (Variables|Gameplay|GetInfos)))) 0))))

(fn Mortgageprice
  (return (/ (Get|GetPrice) 2)))

(fn GetPrice
  (return (Utilities|Struct|BreakST_SquareData (Variables|Gameplay|GetInfos))))

(fn UnmortgagePrice
  (bind _price (Mortgage|Mortgageprice))
  (return (+ (/ _price 10) _price)))

(fn IsBuyable
  (bind _type (Get|GetType))
  (return (and (Math|Boolean|ORBoolean (Utilities|Enum|Equal(Enum) _type "NewEnumerator1") (Utilities|Enum|Equal(Enum) _type "NewEnumerator5") (Utilities|Enum|Equal(Enum) _type "NewEnumerator6")) (== (Variables|Gameplay|GetPlayerOwner) -1))))

(fn GetType
  (return (Utilities|Struct|BreakST_SquareData (Variables|Gameplay|GetInfos))))

(fn GetColor
  (return (Utilities|Struct|BreakST_SquareData (Variables|Gameplay|GetInfos))))

(fn GetName
  (return (Utilities|Struct|BreakST_SquareData (Variables|Gameplay|GetInfos))))

(fn CanBuy
  (params (PlayerId :type Integer))
  (return (and (GamePlay|IsBuyable) (Default|CanPay (Default|GetPlayer (.AsGS%20Game (Utilities|Casting|CastToGS_Game (Game|GetGameState))) PlayerId) (Get|GetPrice)))))

(fn GetHousePrice
  (return (Utilities|Struct|BreakST_RentPrices (.Value (Utilities|Map|Find (Variables|/Game/Monopoly/Levels/Game/Blueprints/Board/BP_Board.BP_Board_C|GetRentPrices (Utilities|GetBoard)) (Variables|Setup|GetN))))))

(fn CanBuildHouse
  (params (PlayerIndex :type Integer))
  (return (Math|Boolean|ANDBoolean (Utilities|Enum|Equal(Enum) (Get|GetType) "NewEnumerator1") (.IsOwner (GamePlay|OwnershipStatus PlayerIndex)) (|AssessPlayerCanPay PlayerIndex) (Default|IsMonopoly (Utilities|GetBoard) (Variables|Setup|GetN)) (not (Variables|Gameplay|GetHotel)) (|No2HousesDifferences) (not (Default|AnyMortgagedinColor (Utilities|GetBoard) (Get|GetColor))))))

(fn BuildHouse
  (bind _houses (Variables|Gameplay|GetHouses))
  (if (== _houses 4)
    (Variables|Gameplay|SetHotel true)
    (else
      (Math|Integer|IncrementInt _houses))))

(fn SellHouse
  (if (Variables|Gameplay|GetHotel)
    (Variables|Gameplay|SetHotel false)
    (else
      (Math|Integer|DecrementInt (Variables|Gameplay|GetHouses)))))

(fn CanSellHouse
  (params (PlayerIndex :type Integer))
  (return (Math|Boolean|ANDBoolean (.IsOwner (GamePlay|OwnershipStatus PlayerIndex)) (Default|IsMonopoly (Utilities|GetBoard) (Variables|Setup|GetN)) (Math|Conversions|ToBoolean(Integer) (Variables|Gameplay|GetHouses)) (|No2HousesDifference))))

(fn Rent
  (bind _returnvalue (Game|GetGameState))
  (bind _type (Get|GetType))
  (bind _board (Utilities|GetBoard))
  (bind _board_2 (Utilities|GetBoard))
  (bind _board_3 (Utilities|GetBoard))
  (bind _playerowner (Variables|Gameplay|GetPlayerOwner))
  (bind _n (Variables|Setup|GetN))
  (bind _asgs_game (Utilities|Casting|CastToGS_Game _returnvalue))
  (bind _asps_game (Utilities|GetPlayer _playerowner))
  (bind _rentprices (Variables|/Game/Monopoly/Levels/Game/Blueprints/Board/BP_Board.BP_Board_C|GetRentPrices _board))
  (bind _diceboxref (Variables|/Game/Monopoly/Levels/Game/Blueprints/Board/BP_Board.BP_Board_C|GetDiceBoxRef _board_3))
  (bind _value (Default|ReadDice _diceboxref))
  (bind _value_2 (Utilities|Map|Find _rentprices _n))
  (bind _biggerfine (Variables|/Game/Monopoly/Levels/Game/Blueprints/GS_Game.GS_Game_C|GetBiggerFine _asgs_game))
  (bind _properties (Variables|/Game/Monopoly/Levels/Game/Blueprints/PS_Game.PS_Game_C|GetProperties _asps_game))
  (bind (_site _house1 _house2 _house3 _house4 _hotel) (Utilities|Struct|BreakST_RentPrices _value_2))
  (bind _count (Default|CountType _board_2 _properties _type))
  (switch Utilities|FlowControl|Switch|SwitchonEN_SquareType (Get|GetType)
    (:NewEnumerator1
      (switch int (Variables|Gameplay|GetHouses)
        (:0
          (if (Default|IsMonopoly (Utilities|GetBoard) (Variables|Setup|GetN))
            (return (* _site 2))
            (else
              (return _site))))
        (:1
          (return _house1))
        (:2
          (return _house2))
        (:3
          (return _house3))
        (:4
          (if (Variables|Gameplay|GetHotel)
            (return _hotel)
            (else
              (return _house4))))))
    (:NewEnumerator5
      (for _index (range 2 _count)
        (LocalVariables|SetL_Railroad (* (LocalVariables|GetL_Railroad) 2)))
      (if _biggerfine
        (return (* (LocalVariables|GetL_Railroad) 2))
        (else
          (return (LocalVariables|GetL_Railroad)))))
    (:NewEnumerator6
      (if (and (== _count 1) (not _biggerfine))
        (return (* _value 4))
        (else
          (return (* _value 10)))))))

(fn CanUnmortgage
  (params (PlayerId :type Integer))
  (return (and (.IsOwner (GamePlay|OwnershipStatus PlayerId)) (Default|CanPay (Utilities|GetPlayer PlayerId) (Mortgage|UnmortgagePrice)))))