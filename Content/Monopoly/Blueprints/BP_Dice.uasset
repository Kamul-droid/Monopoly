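; BP_Dice is a dice actor in the Monopoly game.
; On BeginPlay it gathers six sphere components, Sphere through Sphere5, into SphereArray.
; It contains no roll or face-detection logic, and nothing in its graphs reads the array.
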(event EventBeginPlay
  (bind _spherearray (Variables|Setup|GetsphereArray))
  (Utilities|Array|Add _spherearray (Variables|Default|GetSphere))
  (Utilities|Array|Add _spherearray (Variables|Default|GetSphere1))
  (Utilities|Array|Add _spherearray (Variables|Default|GetSphere2))
  (Utilities|Array|Add _spherearray (Variables|Default|GetSphere3))
  (Utilities|Array|Add _spherearray (Variables|Default|GetSphere4))
  (Utilities|Array|Add _spherearray (Variables|Default|GetSphere5)))

(event Collision|EventActorBeginOverlap
  (params (OtherActor :type Actor%20Object%20Reference)))

(event EventTick
  (params (DeltaSeconds :type Float%20%28single-precision%29)))

(fn ConstructionScript)