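; BP_JailSquare is the jail square on the Monopoly board, a child square Blueprint with a separate set of spots for jailed pawns.
; InitPositions extends the parent's setup by gathering four jail position components into an array.
; OccupyLocation re-runs that setup, picks jail or regular positions by the InJail flag, then records the first free index in the shared Occupied map and returns that spot's world location.
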(event EventBeginPlay)

(event Collision|EventActorBeginOverlap
  (params (OtherActor :type Actor%20Object%20Reference))
  (|CallParentFunction OtherActor) ; This node is disabled and will not be called.\nDrag off pins to build functionality.
)

(event EventTick
  (params (DeltaSeconds :type Float%20%28single-precision%29))
  (|CallParentFunction DeltaSeconds) ; This node is disabled and will not be called.\nDrag off pins to build functionality.
)

(fn ConstructionScript
  (|CallParentFunction))

(fn InitPositions
  (|CallParentFunction)
  (Variables|Default|SetJailPositions (Utilities|Array|MakeArray (Variables|Default|GetJailPosition) (Variables|Default|GetJailPosition1) (Variables|Default|GetJailPosition2) (Variables|Default|GetJailPosition3))))

(fn OccupyLocation
  (params (Pawn :type PN%20Game%20Object%20Reference) (bInJail :type Boolean))
  ;[1 1 1] This is a very dirty fix
  (CallFunction|InitPositions)
  (if bInJail
    (LocalVariables|SetL_PositionsArray (Variables|Default|GetJailPositions))
    (else
      (LocalVariables|SetL_PositionsArray (Variables|Default|GetPositions))))
  (for (_array_element _array_index) (LocalVariables|GetL_PositionsArray)
    (bind _values (Utilities|Map|Values (Variables|Default|GetOccupied)))
    (if (== (Utilities|Array|FindItem _values _array_index) -1)
      (Utilities|Map|Add (Variables|Default|GetOccupied) 0 _array_index)
      (return (Transformation|GetWorldLocation _array_element)))))