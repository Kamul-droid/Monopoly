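; Player controller for the Monopoly menu level that brings up the main menu UI.
; On BeginPlay it creates the UI_MenuMain widget, adds it to the viewport and stores a reference to it.
; If MonopolyGameInstance already holds a valid online user ID, it calls FetchPlayerStatsMessage on the game instance and switches the menu to page 1.
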(event EventBeginPlay
  (bind _returnvalue (UserInterface|CreateWidget "/Game/Monopoly/Levels/Menu/UI_MenuMain.UI_MenuMain_C"))
  (UserInterface|Viewport|AddtoViewport _returnvalue 0)
  (Variables|Default|SetUIMain _returnvalue)
  (if (!= (Utilities|Struct|BreakST_PlayerStats (Variables|/Game/Monopoly/Levels/AllLevels/MonopolyGameInstance.MonopolyGameInstance_C|GetOnlineStats (.AsMonopoly%20Game%20Instance (Utilities|Casting|CastToMonopolyGameInstance (Game|GetGameInstance))))) -1)
    (Class|MonopolyGameInstanceInterface|FetchPlayerStats(Message) (Game|GetGameInstance))
    (Default|Switchto (Variables|Default|GetUIMain) 1)))

(fn ConstructionScript)