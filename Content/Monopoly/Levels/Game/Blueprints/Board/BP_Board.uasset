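; BP_Board is the Monopoly board actor that indexes the level's squares and answers rule queries about them.
; On BeginPlay it caches the dice box and stores each BP_Square by its number, filling its info from defaults.
; Helpers find the next square of a type with wraparound, detect monopolies against the owner's properties, and check building ranges and mortgages per color.
; It also toggles the selected square, updates markers and signals the change.
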(event EventBeginPlay
  (Setup|Init))

(fn ConstructionScript)

(fn Init
  (Setup|SetDiceBoxRef)
  (Setup|SetSquaresRefs))

(fn SetSquaresRefs
  (if (== (Utilities|Array|Length (Variables|References|GetSquaresRef)) 0)
    (bind _outactors (Actor|GetAllActorsOfClass "/Game/Monopoly/Levels/Game/Blueprints/Board/BP_Square.BP_Square_C"))
    (for _array_element _outactors
      (Variables|/Game/Monopoly/Levels/Game/Blueprints/Board/BP_Square.BP_Square_C|SetInfos _array_element (Utilities|Array|Get(acopy) (Variables|Default|GetSquaredefaults) (Variables|/Game/Monopoly/Levels/Game/Blueprints/Board/BP_Square.BP_Square_C|GetN _array_element)))
      (Utilities|Array|SetArrayElem (Variables|References|GetSquaresRef) (Variables|/Game/Monopoly/Levels/Game/Blueprints/Board/BP_Square.BP_Square_C|GetN _array_element) _array_element true))))

(fn Square
  (params (Position :type Integer))
  (return (Utilities|Array|Get(acopy) (Variables|References|GetSquaresRef) Position)))

(fn NextOfType
  (params (Type :type EN_SquareType%20Enum :default "NewEnumerator3") (From :type Integer))
  (bind _squaresref (Variables|References|GetSquaresRef))
  (bind _returnvalue (Utilities|Array|Length _squaresref))
  ;[1 1 1 1 12] Local variable for cleaner management
  (LocalVariables|SetTypeToCheck Type)
  ;[1 1 1 1 12] Goes from x+1 to x
  (for _index (range (+ From 1) (+ From _returnvalue))
    (if (Utilities|Enum|Equal(Enum) (LocalVariables|GetTypeToCheck) (Utilities|Struct|BreakST_SquareData (Variables|/Game/Monopoly/Levels/Game/Blueprints/Board/BP_Square.BP_Square_C|GetInfos (Utilities|Array|Get(acopy) (Variables|References|GetSquaresRef) (Math|Integer|%(Integer) _index _returnvalue)))))
      (return (Math|Integer|%(Integer) _index _returnvalue)))))

(fn CountColor
  (params (Squares :type Array%20of%20BP%20Square%20Object%20References) (Color :type EN_Color%20Enum :default "NewEnumerator0"))
  (for _array_element Squares
    (if (Utilities|Enum|Equal(Enum) Color (Utilities|Struct|BreakST_SquareData (Variables|/Game/Monopoly/Levels/Game/Blueprints/Board/BP_Square.BP_Square_C|GetInfos _array_element)))
      (Math|Integer|IncrementInt (LocalVariables|GetL_Count))))
  (return (LocalVariables|GetL_Count)))

(fn IsMonopoly
  (params (Square :type Integer))
  (bind _square (Gameplay|Square Square))
  (bind _infos (Variables|/Game/Monopoly/Levels/Game/Blueprints/Board/BP_Square.BP_Square_C|GetInfos _square))
  (bind _playerowner (Variables|/Game/Monopoly/Levels/Game/Blueprints/Board/BP_Square.BP_Square_C|GetPlayerOwner _square))
  (bind _color (Utilities|Struct|BreakST_SquareData _infos))
  (if (!= _playerowner -1)
    (return (== (Gameplay|CountColor (Variables|References|GetSquaresRef) _color) (Gameplay|CountColor (Variables|/Game/Monopoly/Levels/Game/Blueprints/PS_Game.PS_Game_C|GetProperties (Default|GetPS (.AsGS%20Game (Utilities|Casting|CastToGS_Game (Game|GetGameState))) _playerowner)) _color)))
    (else
      (return false))))

(fn CountType
  (params (Squares :type Array%20of%20BP%20Square%20Object%20References) (SquareType :type EN_SquareType%20Enum :default "NewEnumerator3"))
  (for _array_element Squares
    (if (Utilities|Enum|Equal(Enum) SquareType (Utilities|Struct|BreakST_SquareData (Variables|/Game/Monopoly/Levels/Game/Blueprints/Board/BP_Square.BP_Square_C|GetInfos _array_element)))
      (Math|Integer|IncrementInt (LocalVariables|GetL_Count))))
  (return (LocalVariables|GetL_Count)))

(fn SetDiceBoxRef
  (Utilities|IsValid (Variables|References|GetDiceBoxRef)
    (:Is%20Not%20Valid
      (bind _outactors (Actor|GetAllActorsOfClass "/Game/Monopoly/Levels/Game/Blueprints/BP_DiceBox.BP_DiceBox_C"))
      (Variables|References|SetDiceBoxRef (Utilities|Array|Get(acopy) _outactors)))))

(fn MinMaxHousesinColor
  (params (Color :type EN_Color%20Enum :default "NewEnumerator0"))
  (for _array_element (Variables|References|GetSquaresRef)
    (if (Utilities|Enum|Equal(Enum) (Utilities|Struct|BreakST_SquareData (Variables|/Game/Monopoly/Levels/Game/Blueprints/Board/BP_Square.BP_Square_C|GetInfos _array_element)) Color)
      (LocalVariables|SetL_Houses (+ (Variables|/Game/Monopoly/Levels/Game/Blueprints/Board/BP_Square.BP_Square_C|GetHouses _array_element) (Math|Conversions|ToInteger(Boolean) (Variables|/Game/Monopoly/Levels/Game/Blueprints/Board/BP_Square.BP_Square_C|GetHotel _array_element))))
      (LocalVariables|SetL_Low (Math|Integer|Min(Integer) (LocalVariables|GetL_Low) (LocalVariables|GetL_Houses)))
      (LocalVariables|SetL_High (Math|Integer|Max(Integer) (LocalVariables|GetL_High) (LocalVariables|GetL_Houses)))))
  (return (LocalVariables|GetL_High) (LocalVariables|GetL_Low)))

(fn SelectSquare
  (params (Square :type Integer))
  (if (== Square (Variables|Default|GetSelected))
    (Variables|Default|SetSelected -1)
    (else
      (Variables|Default|SetSelected Square)))
  (CallFunction|UpdateSquares)
  (Default|CallSquareSelected))

(fn UpdateSquares
  (for _array_element (Variables|References|GetSquaresRef)
    (Default|SetMarkerVisible _array_element (== (Variables|/Game/Monopoly/Levels/Game/Blueprints/Board/BP_Square.BP_Square_C|GetN _array_element) (Variables|Default|GetSelected)))))

(fn AnyMortgagedinColor
  (params (Color :type EN_Color%20Enum :default "NewEnumerator0"))
  (for _array_element (Variables|References|GetSquaresRef)
    (if (and (Variables|/Game/Monopoly/Levels/Game/Blueprints/Board/BP_Square.BP_Square_C|GetMortgaged _array_element) (Utilities|Enum|Equal(Enum) (Default|GetColor _array_element) Color))
      (return true)))
  (return false))