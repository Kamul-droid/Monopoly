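; BP_SquareThin is a Monopoly board square that displays the houses and hotel built on it.
; BeginPlay gathers the four house meshes and the hotel mesh into an ordered array.
; SRV-ShowHouses adds the Hotel flag to the house count and passes the total to M-ShowHouses, apparently a server-to-multicast pair.
; M-ShowHouses makes that many meshes visible from the start of the array and hides the rest.
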(event Custom|SRV%20-%20ShowHouses
  (CallFunction|M-ShowHouses (+ (Variables|Default|GetHouses) (Math|Conversions|ToInteger(Boolean) (Variables|Default|GetHotel)))))

(event Custom|M%20-%20ShowHouses
  (params (B :type Integer))
  (for (_array_element _array_index) (Variables|Default|GetHousesMeshes)
    (Rendering|SetVisibility _array_element (<= (+ _array_index 1) B) false)))

(event EventBeginPlay
  (|CallParentFunction)
  (Variables|Default|SetHousesMeshes (Utilities|Array|MakeArray (Variables|Default|GetHouse1) (Variables|Default|GetHouse2) (Variables|Default|GetHouse3) (Variables|Default|GetHouse4) (Variables|Default|GetHotelMesh))))

(event Collision|EventActorBeginOverlap
  (params (OtherActor :type Actor%20Object%20Reference))
  (|CallParentFunction OtherActor) ; This node is disabled and will not be called.\nDrag off pins to build functionality.
)

(event EventTick
  (params (DeltaSeconds :type Float%20%28single-precision%29))
  (|CallParentFunction DeltaSeconds) ; This node is disabled and will not be called.\nDrag off pins to build functionality.
)

(fn ConstructionScript
  (|CallParentFunction))