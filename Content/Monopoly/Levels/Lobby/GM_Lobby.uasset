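; Lobby game mode for a multiplayer Monopoly game that gathers players and starts the match once the session fills.
; On login it tracks each lobby controller, refreshes all clients after a retriggerable delay, then compares the player count to the session's connection limit.
; Surplus players are kicked as "Server Full"; at capacity it updates the session, shows a start message, clears client UI and server-travels to MapMulti.
; Logout removes the controller from the list.
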(event EventPostLogin
  (params (NewPlayer :type Player%20Controller%20Object%20Reference))
  (bind _aspc_lobby (Utilities|Casting|CastToPC_Lobby NewPlayer))
  (bind _pcsref (Variables|Default|GetPCsRef))
  (bind _returnvalue (Utilities|Array|Length _pcsref))
  (Default|InitCLIENT _aspc_lobby)
  (Utilities|Array|AddUnique (Variables|Default|GetPCsRef) _aspc_lobby)
  (Utilities|FlowControl|RetriggerableDelay 2.0)
  (CallFunction|RefreshAll)
  (bind (_numconnections _numprivateconnections _bislan _bisdedicated _ballowinvites _ballowjoininprogress _bisanticheatenabled _builduniqueid _extrasettings) (Class|AdvancedSessionsLibrary|GetSessionSettings)
    (:OnSuccess
      (if (> _returnvalue _numconnections)
        (bind (_arrayindex _arrayelement) (Utilities|Array|ReverseforEachLoop (Variables|Default|GetPCsRef))
          (:LoopBody
            (if (>= _arrayindex _numconnections)
              (Class|AdvancedSessionsLibrary|KickPlayer _arrayelement "Server Full")))
          (:Completed
            (|UpdateSession _extrasettings _numconnections 0 false false false true false :!label _label
              (:OnSuccess
                (CallFunction|StartMessageAll)
                (Utilities|FlowControl|Delay 2.0)
                (CallFunction|ClearAll)
                (Development|ExecuteConsoleCommand "serverTravel MapMulti" 0)))))
        (elif (== _returnvalue _numconnections)
          (goto _label))))))

(event EventOnLogout
  (params (ExitingController :type Controller%20Object%20Reference))
  (bind _aspc_lobby (Utilities|Casting|CastToPC_Lobby ExitingController))
  (Utilities|Array|RemoveItem (Variables|Default|GetPCsRef) _aspc_lobby))

(fn ConstructionScript)

(fn RefreshAll
  (for _array_element (Variables|Default|GetPCsRef)
    (Default|RefreshOthersCLIENT _array_element)))

(fn StartMessageAll
  (for _array_element (Variables|Default|GetPCsRef)
    (Default|StartMessageCLIENT _array_element)))

(fn ClearAll
  (for _array_element (Variables|Default|GetPCsRef)
    (Default|ClearUICLIENT _array_element)))