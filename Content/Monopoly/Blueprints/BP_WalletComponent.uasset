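; Wallet component for Monopoly that handles player cash as maps of bill denomination to quantity, with helpers to build, total, adjust and combine wallets.
; PayAmount greedily pays from largest bill down, returning both the payment and the payer's updated wallet.
; Any shortfall makes BreakBillForAmount split the smallest larger bill through hardcoded change rules, then PayAmount recurses.
; Payment assumes sufficient funds, which CanPay checks separately against the wallet total.
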(event EventBeginPlay)

(event EventTick
  (params (DeltaSeconds :type Float%20%28single-precision%29)))

(fn GetWalletTotal
  (params (Wallet :type Map%20of%20Integers%20to%20Integers))
  (for _array_element (Variables|ReadOnly|GetValidBillsDescending)
    (if (.ReturnValue (Utilities|Map|Find Wallet _array_element))
      (LocalVariables|SetTotalAmount (+ (LocalVariables|GetTotalAmount) (* (.Value (Utilities|Map|Find Wallet _array_element)) _array_element)))))
  (return (LocalVariables|GetTotalAmount)))

(fn PayAmount
  (params (PlayerWallet :type Map%20of%20Integers%20to%20Integers) (Amount :type Integer))
  (LocalVariables|SetDebitWallet PlayerWallet)
  (LocalVariables|SetAmountToPay Amount)
  (for _array_element (Variables|ReadOnly|GetValidBillsDescending)
    (bind _output_get (LocalVariables|SetCurrentBillValue _array_element))
    (LocalVariables|SetCurrentBillQuantity (.Value (Utilities|Map|Find (LocalVariables|GetDebitWallet) _output_get)))
    (while (and (>= (LocalVariables|GetAmountToPay) (LocalVariables|GetCurrentBillValue)) (> (LocalVariables|GetCurrentBillQuantity) 0))
      (LocalVariables|SetAmountToPay (- (LocalVariables|GetAmountToPay) (LocalVariables|GetCurrentBillValue)))
      (Math|Integer|DecrementInt (LocalVariables|GetCurrentBillQuantity)))
    (Utilities|Map|Add (LocalVariables|GetPaidBills) (LocalVariables|GetCurrentBillValue) (- (.Value (Utilities|Map|Find (LocalVariables|GetDebitWallet) (LocalVariables|GetCurrentBillValue))) (LocalVariables|GetCurrentBillQuantity))) ; Adds to the payment bill
    (Utilities|Map|Add (LocalVariables|GetDebitWallet) (LocalVariables|GetCurrentBillValue) (LocalVariables|GetCurrentBillQuantity)) ; Removes from the payer's bills
  )
  (if (== (LocalVariables|GetAmountToPay) 0)
    (return (LocalVariables|GetPaidBills) (LocalVariables|GetDebitWallet))
    (else
      ;[1 1 1] Note: this assumes the player has enough money, the function should never be called if the player can't pay
      (bind _outputwallet (GamePlay|BreakBillforAmount (LocalVariables|GetDebitWallet) (LocalVariables|GetAmountToPay)))
      (bind (_payment _payerwallet) (GamePlay|PayAmount _outputwallet (LocalVariables|GetAmountToPay)))
      (LocalVariables|SetDebitWallet _payerwallet)
      (bind _combinedwallet (GamePlay|CombineWallets _payment (LocalVariables|GetPaidBills)))
      (return _combinedwallet (LocalVariables|GetDebitWallet)))))

(fn CombineWallets
  (params (Wallet1 :type Map%20of%20Integers%20to%20Integers) (Wellet2 :type Map%20of%20Integers%20to%20Integers))
  (for _array_element (Variables|ReadOnly|GetValidBillsDescending)
    (Utilities|Map|Add (LocalVariables|GetTempCombinedWallet) _array_element (+ (.Value (Utilities|Map|Find Wallet1 _array_element)) (.Value (Utilities|Map|Find Wellet2 _array_element)))))
  (return (LocalVariables|GetTempCombinedWallet)))

(fn BreakBillforAmount
  (params (Wallet :type Map%20of%20Integers%20to%20Integers) (Amount :type Integer))
  (LocalVariables|SetPlayerWallet Wallet)
  (for _array_element (Variables|ReadOnly|GetValidBillsDescending)
    (if (and (> (.Value (Utilities|Map|Find (LocalVariables|GetPlayerWallet) _array_element)) 0) (> _array_element Amount))
      (LocalVariables|SetLowestAbove _array_element)))
  (bind _walletreturn (GamePlay|AddtoWallet (LocalVariables|GetPlayerWallet) (LocalVariables|GetLowestAbove) -1))
  (LocalVariables|SetPlayerWallet _walletreturn)
  (switch string (Utilities|String|ToString(Integer) (LocalVariables|GetLowestAbove)) ; Screw this.
    (:500
      (bind _walletreturn_2 (GamePlay|AddtoWallet (LocalVariables|GetPlayerWallet) 100 5))
      (return _walletreturn_2))
    (:100
      (bind _walletreturn_3 (GamePlay|AddtoWallet (LocalVariables|GetPlayerWallet) 50 2))
      (return _walletreturn_3))
    (:50
      (bind _walletreturn_4 (GamePlay|AddtoWallet (LocalVariables|GetPlayerWallet) 20 2))
      (bind _walletreturn_5 (GamePlay|AddtoWallet _walletreturn_4 10 1))
      (return _walletreturn_5))
    (:20
      (bind _walletreturn_6 (GamePlay|AddtoWallet (LocalVariables|GetPlayerWallet) 10 2))
      (return _walletreturn_6))
    (:10
      (bind _walletreturn_7 (GamePlay|AddtoWallet (LocalVariables|GetPlayerWallet) 5 2))
      (return _walletreturn_7))
    (:5
      (bind _walletreturn_8 (GamePlay|AddtoWallet (LocalVariables|GetPlayerWallet) 1 5))
      (return _walletreturn_8))))

(fn AddtoWallet
  (params (Wallet :type Map%20of%20Integers%20to%20Integers) (BillValue :type Integer) (Amount :type Integer))
  (Utilities|Map|Add Wallet BillValue (+ (.Value (Utilities|Map|Find Wallet BillValue)) Amount))
  (return Wallet))

(fn CanPay
  (params (Amount :type Integer) (Wallet :type Map%20of%20Integers%20to%20Integers))
  (return (<= Amount (GamePlay|GetWalletTotal Wallet))))

(fn MakeWallet
  (params (500 :type Integer) (100 :type Integer) (50 :type Integer) (20 :type Integer) (10 :type Integer) (5 :type Integer) (1 :type Integer))
  (return (Utilities|Map|MakeMap 500 500 100 100 50 50 20 20 10 10 5 5 1 1)))