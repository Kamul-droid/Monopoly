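; Lobby player controller for the Monopoly game that sets the player's online name and owns the lobby screen.
; On BeginPlay it passes the GameInstance's online name to a server event that writes it to PS_Lobby, then creates the UI_LobbyMain widget.
; Client events forward text changes, player refreshes and removal to that widget.
; InitCLIENT polls on a looping timer until the GameState's PlayerArray is populated, then only stops the timer.
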(event Custom|ClearUI%20CLIENT
  (Widget|RemovefromParent (Variables|Default|GetLobbyMainRef)))

(event Custom|SRV%20-%20SetOnlineName
  (params (Name :type String))
  (Variables|/Game/Monopoly/Levels/Lobby/PS_Lobby.PS_Lobby_C|SetName (Utilities|GetPS) Name))

(event Custom|RefreshOthers%20CLIENT
  (Default|RefreshOthers (Variables|Default|GetLobbyMainRef)))

(event Custom|GSIsHere
  (if (Math|Conversions|ToBoolean(Integer) (Utilities|Array|Length (Variables|/Script/Engine.GameStateBase|GetPlayerArray (Game|GetGameState))))
    (Utilities|Time|ClearandInvalidateTimerbyHandle (stale Custom|Init%20CLIENT _returnvalue))))

(event Custom|Init%20CLIENT
  (bind _returnvalue (Utilities|Time|SetTimerbyEvent (delegate Custom|GSIsHere) 0.1 true)))

(event Custom|StartMessage%20CLIENT
  (Default|Changetext (Variables|Default|GetLobbyMainRef)))

(event EventBeginPlay
  (CallFunction|SRV-SetOnlineName (Variables|/Game/Monopoly/Levels/AllLevels/MonopolyGameInstance.MonopolyGameInstance_C|GetOnlineName (Utilities|GetGI)))
  (CallFunction|SetUI))

(fn ConstructionScript)

(fn SetUI
  (bind _returnvalue (UserInterface|CreateWidget "/Game/Monopoly/Levels/Lobby/UI_LobbyMain.UI_LobbyMain_C" (Game|GetPlayerController 0)))
  (UserInterface|Viewport|AddtoViewport _returnvalue 0)
  (Variables|Default|SetLobbyMainRef _returnvalue))