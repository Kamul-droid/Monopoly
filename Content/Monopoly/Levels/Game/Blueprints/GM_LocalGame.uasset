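; Game mode for local multiplayer Monopoly, hosting all players on one machine and driving the turn order.
; On BeginPlay it creates local players with possessed pawns, sets up game state and rules (chat off) and player UIs, then picks a random starting player.
; CycleTurns resets per-turn state, triggers auction checks, skips bankrupt players and toggles each player's UI.
; The turn counter increments whenever play returns to the starting player.
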(event Custom|StartGame
  (bind _asgs_game (Utilities|GetGS))
  (bind _returnvalue (Class|GameModeBase|GetNumPlayers))
  (Variables|Default|SetActivePlayer (Math|Random|RandomInteger _returnvalue))
  (Default|PickStartingPlayer _asgs_game (Variables|/Script/Engine.PlayerState|GetPlayerId (Utilities|GetActivePS)))
  (CallFunction|SetActivePlayerTurn true)
  (Variables|/Game/Monopoly/Levels/Game/Blueprints/GS_Game.GS_Game_C|SetPlaying _asgs_game true))

(event EventBeginPlay
  (CallFunction|SpawnPlayers)
  (CallFunction|SetGameState)
  (CallFunction|SetRules)
  (CallFunction|InitPlayerUIs)
  (CallFunction|StartGame))

(event EventNotifyPlayers
  (params (Notification :type Text))
  (Default|NotifyCLIENT (Utilities|GetActivePC) Notification))

(event EventCycleTurns
  (bind _asgs_game (Utilities|GetGS))
  ;[1 1 1] Turn Cycling
  (Default|ResetTurnSpecific _asgs_game)
  (Class|GSIGame|AuctionifNotBought(Message) _asgs_game)
  (Class|GSIGame|CheckAuctions(Message) _asgs_game)
  (CallFunction|SetActivePlayerTurn false)
  (CallFunction|SwapActivePlayer :!label _label)
  (if (Variables|/Game/Monopoly/Levels/Game/Blueprints/PS_Game.PS_Game_C|GetbBankrupt (Utilities|GetActivePS))
    (goto _label)
    (else
      (CallFunction|SetActivePlayerTurn true))))

(fn ConstructionScript)

(fn SpawnPlayers
  (for _index (range 0 (- (Variables|Default|GetMaxPlayers) 1))
    (Class|GameplayStatics|CreatePlayer _index)
    (bind _returnvalue (Game|SpawnActorfromClass "/Game/Monopoly/Levels/Game/Blueprints/PN_Game.PN_Game_C" (Math|Transform|MakeTransform "0, 0, 0") "AlwaysSpawn" 0 0))
    (Pawn|Possess (Game|GetPlayerController _index) _returnvalue)
    (Utilities|Array|Add (Variables|Default|GetPCs) (.AsPC%20Game (Utilities|Casting|CastToPC_Game (Game|GetPlayerController _index))))))

(fn SetGameState
  (Variables|/Game/Monopoly/Levels/Game/Blueprints/GS_Game.GS_Game_C|SetNumPlayers (Utilities|GetGS) (Variables|Default|GetMaxPlayers)))

(fn SwapActivePlayer
  (bind _asgs_game (Utilities|GetGS))
  (bind _asps_game (Utilities|GetActivePS))
  (bind _asgs_game_2 (Utilities|GetGS))
  (Variables|Default|SetActivePlayer (Math|Integer|%(Integer) (+ (Variables|Default|GetActivePlayer) 1) (Variables|/Game/Monopoly/Levels/Game/Blueprints/GS_Game.GS_Game_C|GetNumPlayers _asgs_game_2)))
  (Variables|/Game/Monopoly/Levels/Game/Blueprints/GS_Game.GS_Game_C|SetActivePlayerId _asgs_game (Variables|/Script/Engine.PlayerState|GetPlayerId _asps_game))
  (if (== (Variables|/Script/Engine.PlayerState|GetPlayerId _asps_game) (Variables|/Game/Monopoly/Levels/Game/Blueprints/GS_Game.GS_Game_C|GetStartingPlayer _asgs_game_2))
    (Math|Integer|IncrementInt (Variables|/Game/Monopoly/Levels/Game/Blueprints/GS_Game.GS_Game_C|GetTurn _asgs_game))))

(fn SetActivePlayerTurn
  (params (MyTurn :type Boolean))
  (bind _aspc_game (Utilities|GetActivePC))
  (bind _asps_game (Utilities|GetActivePS))
  (if MyTurn
    (Default|StartTurnCLIENT _aspc_game)
    (Default|ShowPlayerUI _aspc_game)
    (Class|PSIGame|SetStatus(Message) _asps_game "NewEnumerator1")
    (else
      (Default|EndTurnCLIENT _aspc_game)
      (Default|HidePlayerUI _aspc_game)
      (Class|PSIGame|SetStatus(Message) _asps_game "NewEnumerator0"))))

(fn SetRules
  (Variables|/Game/Monopoly/Levels/Game/Blueprints/GS_Game.GS_Game_C|SetChatEnabled (Utilities|GetGS) false))

(fn InitPlayerUIs
  (for _array_element (Variables|Default|GetPCs)
    (Default|SetUIRef _array_element)))