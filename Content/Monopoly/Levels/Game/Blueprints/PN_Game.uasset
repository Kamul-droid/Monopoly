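; PN_Game is the Monopoly game level's camera pawn, which the player rotates horizontally.
; The RotatePlayerCamera axis input subtracts its value from the Azimuth component's relative yaw, holding pitch and roll at zero.
; The step is not scaled by delta time, so rotation speed depends on frame rate.
; The construction script is empty, and leftover sine nodes in the event graph are unconnected.
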(event Input|AxisEvents|InputAxisRotatePlayerCamera
  (params (AxisValue :type Float%20%28single-precision%29))
  (if (!= AxisValue 0.0)
    (Transformation|SetRelativeRotation (Variables|Default|GetAzimuth) (Math|Rotator|MakeRotator 0.0 0.0 (- (.Yaw (Math|Rotator|BreakRotator (Variables|/Script/Engine.SceneComponent|GetRelativeRotation (Variables|Default|GetAzimuth)))) AxisValue)) false false)))

(fn ConstructionScript)