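; Game mode for the Monopoly multiplayer lobby, tracking joined player controllers and starting the match once everyone is ready.
; Joins and leaves update the controller list and refresh every client's lobby, and players beyond four are kicked.
; CheckCanStart requires at least two ready players, updates the session's public connections, shows a countdown message, then rechecks readiness before server-traveling to MapMulti.
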(event Custom|CheckCanStart
  (if (CallFunction|AllReady)
    (|UpdateSession 0 (Utilities|Array|Length (Variables|Default|GetPCsRef)) 0 false false false true false
      (:OnSuccess
        (CallFunction|MessageAll "Game Starting Soon")
        (Utilities|FlowControl|Delay 2.0)
        (if (CallFunction|AllReady)
          (CallFunction|ClearAll)
          (Development|ExecuteConsoleCommand "serverTravel MapMulti" 0)
          (else
            (CallFunction|MessageAll)))))))

(event EventPostLogin
  (params (NewPlayer :type Player%20Controller%20Object%20Reference))
  (Utilities|Array|AddUnique (Variables|Default|GetPCsRef) (.AsPC%20MP%20Lobby (Utilities|Casting|CastToPC_MP_Lobby NewPlayer)))
  (CallFunction|KickifMoreThan 4)
  (Utilities|FlowControl|RetriggerableDelay 1.0)
  (CallFunction|RefreshAll))

(event EventOnLogout
  (params (ExitingController :type Controller%20Object%20Reference))
  (Utilities|Array|RemoveItem (Variables|Default|GetPCsRef) (.AsPC%20MP%20Lobby (Utilities|Casting|CastToPC_MP_Lobby ExitingController)))
  (CallFunction|RefreshAll))

(fn ConstructionScript)

(fn RefreshAll
  (for _array_element (Variables|Default|GetPCsRef)
    (Default|RefreshOthersCLIENT _array_element)))

(fn MessageAll
  (params (InText :type Text))
  (for _array_element (Variables|Default|GetPCsRef)
    (Default|StartMessageCLIENT _array_element InText)))

(fn ClearAll
  (for _array_element (Variables|Default|GetPCsRef)
    (Default|ClearUICLIENT _array_element)))

(fn KickifMoreThan
  (params (MoreThan :type Integer))
  (if (> (Utilities|Array|Length (Variables|Default|GetPCsRef)) MoreThan)
    (bind (_arrayindex _arrayelement) (Utilities|Array|ReverseforEachLoop (Variables|Default|GetPCsRef))
      (:LoopBody
        (if (>= _arrayindex MoreThan)
          (Class|AdvancedSessionsLibrary|KickPlayer _arrayelement "Server Full"))))))

(fn AllReady
  (for _array_element (Variables|/Script/Engine.GameStateBase|GetPlayerArray (Game|GetGameState))
    (if (or (not (Variables|/Game/Monopoly/Levels/Lobby/MultiPlayer/PS_MP_Lobby.PS_MP_Lobby_C|GetbIsReady (.AsPS%20MP%20Lobby (Utilities|Casting|CastToPS_MP_Lobby _array_element)))) (< (Utilities|Array|Length (Variables|Default|GetPCsRef)) 2))
      (return false)))
  (return true))