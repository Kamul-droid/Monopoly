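; BP_Dice is a dice Blueprint for the Monopoly game level, holding six sphere components.
; On BeginPlay it adds the six spheres, in order, to SphereArray.
; It contains no roll or face-reading logic, and its construction script is empty.
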(event EventBeginPlay
  (bind _spherearray (Variables|Setup|GetsphereArray))
  (Utilities|Array|Add _spherearray (Variables|Default|GetSphere))
  (Utilities|Array|Add _spherearray (Variables|Default|GetSphere1))
  (Utilities|Array|Add _spherearray (Variables|Default|GetSphere2))
  (Utilities|Array|Add _spherearray (Variables|Default|GetSphere3))
  (Utilities|Array|Add _spherearray (Variables|Default|GetSphere4))
  (Utilities|Array|Add _spherearray (Variables|Default|GetSphere5)))

(fn ConstructionScript)