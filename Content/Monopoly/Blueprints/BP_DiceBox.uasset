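; Dice box actor for a Monopoly game that rolls two physics dice and records their values on the player.
; Touching the cube spawns two BP_Dice, which receive random impulses after a short delay.
; Tick then polls velocities until all tracked dice stop.
; Each die's highest marker sphere determines its face value, which is written to BP_Player's DiceValues and printed for debugging.
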(event OnInputTouchBegin(Cube)
  (params (FingerIndex :type ETouchIndex%20Enum :default "Touch1") (TouchedComponent :type Primitive%20Component%20Object%20Reference))
  (bind _cube (Variables|Default|GetCube))
  (bind _cube_2 (Variables|Default|GetCube))
  (bind _dicearray (Variables|Default|GetdiceArray))
  (bind _returnvalue (Transformation|GetWorldLocation _cube))
  (bind _returnvalue_2 (Transformation|GetWorldLocation _cube_2))
  (bind (_x _y _z) (Math|Vector|BreakVector _returnvalue))
  (bind (_x_2 _y_2 _z_2) (Math|Vector|BreakVector _returnvalue_2))
  (bind _returnvalue_3 (Game|SpawnActorfromClass "/Game/Monopoly/Blueprints/BP_Dice.BP_Dice_C" (Math|Transform|MakeTransform (Math|Vector|MakeVector _x_2 (+ _y_2 1e+02) (+ _z_2 5e+01)) "0, 0, 0" "6.000000,6.000000,6.000000") "Undefined" 0 0))
  (Utilities|Array|Add _dicearray _returnvalue_3)
  (bind _returnvalue_4 (Game|SpawnActorfromClass "/Game/Monopoly/Blueprints/BP_Dice.BP_Dice_C" (Math|Transform|MakeTransform (Math|Vector|MakeVector _x (- _y 1e+02) (+ _z 5e+01)) "0, 0, 0" "6.000000,6.000000,6.000000") "Undefined" 0 0))
  (Utilities|Array|Add _dicearray _returnvalue_4)
  (Utilities|FlowControl|Delay 2.0)
  (Physics|AddImpulse (Variables|/Game/Monopoly/Blueprints/BP_Dice.BP_Dice_C|GetDice _returnvalue_3) (Math|Vector|MakeVector (Math|Random|RandomFloatinRange -2e+04 9e+03) (Math|Random|RandomFloatinRange -1e+04 9e+03) (Math|Random|RandomFloatinRange 2e+01 6e+01)) "None" false)
  (Physics|AddImpulse (Variables|/Game/Monopoly/Blueprints/BP_Dice.BP_Dice_C|GetDice _returnvalue_4) (Math|Vector|MakeVector (Math|Random|RandomFloatinRange -2e+02 8.5e+02) (Math|Random|RandomFloatinRange -2e+02 8.5e+02) (Math|Random|RandomFloatinRange 1e+01 1e+02)) "None" false)
  (Utilities|FlowControl|Delay 0.2)
  (Variables|Default|SetisRolling true))

(event EventTick
  (params (DeltaSeconds :type Float%20%28single-precision%29))
  (if (Variables|Default|GetisRolling)
    (bind _array_element (Utilities|Array|ForEachLoopwithBreak (Variables|Default|GetdiceArray) :!label _label)
      (:LoopBody
        (if (Math|Vector|Equal(Vector) (Transformation|GetComponentVelocity (Variables|/Game/Monopoly/Blueprints/BP_Dice.BP_Dice_C|GetDice _array_element)) "0, 0, 0" 0.0001)
          (Variables|Default|SetDiceHaveStoped true)
          (else
            (Variables|Default|SetDiceHaveStoped false)
            (goto _label Break))))
      (:Completed
        (if (Variables|Default|GetDiceHaveStoped)
          (Development|PrintText "Hello")
          (Variables|Default|SetisRolling false)
          (CallFunction|GetHighestFaces))))))

(event EventBeginPlay
  (bind _asbp_player (Utilities|Casting|CastToBP_Player (Game|Player|GetPlayerPawn 0)))
  (Variables|Default|SetPlayerRef _asbp_player))

(fn ConstructionScript)

(fn GetHighestFaces
  (for _array_element (Variables|Default|GetdiceArray)
    (Variables|Default|SetHIghtZ -1e+02)
    (for (_array_element_2 _array_index) (Variables|/Game/Monopoly/Blueprints/BP_Dice.BP_Dice_C|GetsphereArray _array_element)
      (if (> (.Z (Math|Vector|BreakVector (Transformation|GetWorldLocation _array_element_2))) (Variables|Default|GetHIghtZ))
        (Variables|Default|SetHIghtZ (.Z (Math|Vector|BreakVector (Transformation|GetWorldLocation _array_element_2))))
        (Variables|Default|SetHIghestSphere _array_element_2)
        (Variables|Default|Setsphereindex _array_index)))
    (switch int (Variables|Default|Getsphereindex)
      (:0
        (Variables|Default|Setdievalue 5))
      (:1
        (Variables|Default|Setdievalue 4))
      (:2
        (Variables|Default|Setdievalue 3))
      (:3
        (Variables|Default|Setdievalue 6))
      (:4
        (Variables|Default|Setdievalue 1))
      (:5
        (Variables|Default|Setdievalue 2)))
    (Utilities|Array|SetArrayElem (Variables|/Game/Monopoly/Blueprints/BP_Player.BP_Player_C|GetDiceValues (Variables|Default|GetPlayerRef)) (Variables|Default|Getiterator) (Variables|Default|Getdievalue))
    (Math|Integer|IncrementInt (Variables|Default|Getiterator)))
  (CallFunction|PrintValues))

(fn PrintValues
  (for _array_element (Variables|/Game/Monopoly/Blueprints/BP_Player.BP_Player_C|GetDiceValues (Variables|Default|GetPlayerRef))
    (Development|PrintText (Utilities|Text|ToText(Integer) _array_element))))