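; Dice box for the Monopoly game that rolls two physics-simulated BP_Dice and reports their result.
; RollDice replaces the old dice with new spawns and applies random linear and angular impulses.
; Tick waits until both stop moving, then fires SRV-DiceAction to notify the GameState.
; ReadDice maps each die's highest marker sphere to its face value, returning total and doubles, unless SetCheatDice has overridden the result.
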(event Custom|SRV%20-%20DiceAction
  (Class|GSIGame|DiceAction(Message) (Game|GetGameState)))

(event Custom|RollDice
  (bind _returnvalue (Math|Random|RandomFloatinRange 8e+02 1.5e+03))
  (bind _returnvalue_2 (Math|Random|RandomFloat))
  (bind _returnvalue_3 (Math|Random|RandomBool))
  (bind _dicearray (Variables|Default|GetdiceArray))
  (bind _returnvalue_4 (Math|Integer|SelectInt -1 1 _returnvalue_3))
  (bind _returnvalue_5 (* _returnvalue_2 3.6e+02))
  (bind _returnvalue_6 (* _returnvalue_4 _returnvalue))
  (for _array_element _dicearray
    (Actor|DestroyActor _array_element))
  (Utilities|Array|Clear _dicearray)
  (bind _returnvalue_7 (Game|SpawnActorfromClass "/Game/Monopoly/Levels/Game/Blueprints/BP_Dice.BP_Dice_C" (Utilities|GetPositionOffsetandRandomRotationfromMesh (Variables|Default|GetDiceSpawn) "100.000000,50.000000,150.000000") "Undefined" 0 0))
  (Utilities|Array|Add (Variables|Default|GetdiceArray) _returnvalue_7)
  (bind _returnvalue_8 (Game|SpawnActorfromClass "/Game/Monopoly/Levels/Game/Blueprints/BP_Dice.BP_Dice_C" (Utilities|GetPositionOffsetandRandomRotationfromMesh (Variables|Default|GetDiceSpawn) "-100.000000,50.000000,100.000000") "Undefined" 0 0))
  (Utilities|Array|Add (Variables|Default|GetdiceArray) _returnvalue_8)
  (for _array_element_2 (Variables|Default|GetdiceArray)
    (Physics|AddImpulse (Variables|/Game/Monopoly/Levels/Game/Blueprints/BP_Dice.BP_Dice_C|GetDice _array_element_2) (Math|Vector|MakeVector _returnvalue_6 _returnvalue_6 (Math|Random|RandomFloatinRange -2e+02 1e+02)) "None" true)
    (Class|PrimitiveComponent|AddAngularImpulseinDegrees (Variables|/Game/Monopoly/Levels/Game/Blueprints/BP_Dice.BP_Dice_C|GetDice _array_element_2) (Math|Vector|MakeVector _returnvalue_5 _returnvalue_5 _returnvalue_5) "None" true)
    (Utilities|FlowControl|Delay 0.2)
    (Variables|Default|SetisRolling true)))

(event EventTick
  (params (DeltaSeconds :type Float%20%28single-precision%29))
  (if (Variables|Default|GetisRolling)
    (bind _array_element (Utilities|Array|ForEachLoopwithBreak (Variables|Default|GetdiceArray) :!label _label)
      (:LoopBody
        (if (Math|Vector|Equal(Vector) (Transformation|GetComponentVelocity (Variables|/Game/Monopoly/Levels/Game/Blueprints/BP_Dice.BP_Dice_C|GetDice _array_element)) "0, 0, 0" 0.0001)
          (Variables|Default|SetDiceHaveStoped true)
          (else
            (Variables|Default|SetDiceHaveStoped false)
            (goto _label Break))))
      (:Completed
        (if (Variables|Default|GetDiceHaveStoped)
          (Variables|Default|SetisRolling false)
          (CallFunction|SRV-DiceAction))))))

(fn ConstructionScript)

(fn ReadDice
  (bind _dicevalues (LocalVariables|GetDiceValues))
  (bind _dicevalues_2 (LocalVariables|GetDiceValues))
  (bind _output (Utilities|Array|Get(acopy) _dicevalues 1))
  (bind _output_2 (Utilities|Array|Get(acopy) _dicevalues))
  (if (== (Variables|Testing|GetCheatValue) -1)
    (for _array_element (Variables|Default|GetdiceArray)
      (LocalVariables|SetHighestPointZ -1e+02)
      (for (_array_element_2 _array_index) (Variables|/Game/Monopoly/Levels/Game/Blueprints/BP_Dice.BP_Dice_C|GetsphereArray _array_element)
        (if (> (.Z (Math|Vector|BreakVector (Transformation|GetWorldLocation _array_element_2))) (LocalVariables|GetHighestPointZ))
          (LocalVariables|SetHighestPointZ (.Z (Math|Vector|BreakVector (Transformation|GetWorldLocation _array_element_2))))
          (LocalVariables|SetHighestPointIndex _array_index)))
      (switch int (LocalVariables|GetHighestPointIndex)
        (:0
          (Utilities|Array|Add _dicevalues_2 5))
        (:1
          (Utilities|Array|Add _dicevalues_2 4))
        (:2
          (Utilities|Array|Add _dicevalues_2 3))
        (:3
          (Utilities|Array|Add _dicevalues_2 6))
        (:4
          (Utilities|Array|Add _dicevalues_2 1))
        (:5
          (Utilities|Array|Add _dicevalues_2 2))))
    (return (+ _output_2 _output) (== _output_2 _output))
    (else
      (return (Variables|Testing|GetCheatValue) (Variables|Testing|GetCheatDouble)))))

(fn SetCheatDice
  (params (Value :type Integer) (Double :type Boolean))
  (Variables|Testing|SetCheatValue Value)
  (Variables|Testing|SetCheatDouble Double))