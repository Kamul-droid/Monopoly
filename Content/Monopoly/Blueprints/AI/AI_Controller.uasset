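; AI controller for computer players in the Monopoly game, running the BTT_Player behavior tree on possession.
; BeginPlay caches the BP_GameMode reference.
; Every tick it copies the game mode's AiTurn flag into the blackboard's Turn key and clears the flag, so each signal is consumed once.
; ResetTurnInBB provides a way to clear the Endturn key.
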(event EventPossess
  (params (PossessedPawn :type Pawn%20Object%20Reference))
  (AI|RunBehaviorTree "/Game/Monopoly/Blueprints/AI/BTT_Player.BTT_Player"))

(event EventTick
  (params (DeltaSeconds :type Float%20%28single-precision%29))
  (AI|Components|Blackboard|SetValueasBool (AI|GetBlackboard 0) (Variables|Default|GetTurn) (Variables|/Game/Monopoly/Blueprints/BP_GameMode.BP_GameMode_C|GetAiTurn (Variables|References|GetGameModeRef)))
  (Variables|/Game/Monopoly/Blueprints/BP_GameMode.BP_GameMode_C|SetAiTurn (Variables|References|GetGameModeRef) false))

(event EventBeginPlay
  (CallFunction|Init))

(fn ConstructionScript)

(fn Init
  (Utilities|IsValid (Variables|References|GetGameModeRef)
    (:Is%20Not%20Valid
      (bind _asbp_game_mode (Utilities|Casting|CastToBP_GameMode (Game|GetGameMode)))
      (Variables|References|SetGameModeRef _asbp_game_mode))))

(fn ResetTurninBB
  (AI|Components|Blackboard|SetValueasBool (AI|GetBlackboard 0) (Variables|Default|Getendturn) false))