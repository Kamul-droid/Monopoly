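; Monopoly player Blueprint that holds the state of all players and rotates the camera through an Azimuth component's yaw.
; Index-based functions edit player structs: name, wallet, jail state, owned squares and cards, though RemoveCommunityCard adds instead of removing.
; Movement wraps board position at 40 squares and computes a lap flag, and a query totals each player's houses and hotels.
; Initialize and SetPlayerCamera are empty stubs.
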(event Custom|SetPlayerCamera)

(fn ConstructionScript)

(fn Initialize)

(fn RotateCamera
  (params (Axis :type Float%20%28single-precision%29))
  (if (!= Axis 0.0)
    (Transformation|SetRelativeRotation (Variables|Default|GetAzimuth) (Math|Rotator|MakeRotator 0.0 0.0 (+ Axis (.yaw (Variables|/Script/Engine.SceneComponent|GetRelativeRotation (Variables|Default|GetAzimuth))))) false false)))

(fn GetPlayerbyIndex
  (params (Index :type Integer))
  (return (Utilities|PlayerbyIndex Index)))

(fn SetPlayerName
  (params (PlayerIndex :type Integer) (Name :type String))
  (Utilities|Struct|SetmembersinST_Player (Utilities|PlayerbyIndex PlayerIndex) Name))

(fn AdvanceSquares
  (params (PlayerIndex :type Integer) (Squares :type Integer))
  (bind _playerst (Utilities|PlayerbyIndex PlayerIndex))
  (bind _boardposition (Utilities|Struct|BreakST_Player _playerst))
  (bind _returnvalue (+ _boardposition Squares))
  (bind _returnvalue_2 (Math|Integer|%(Integer) _returnvalue 40))
  (Utilities|Struct|SetmembersinST_Player _playerst _returnvalue_2)
  (Variables|GamePlay|SetDidLap (<= _returnvalue_2 _boardposition)))

(fn AdvancetoSquare
  (params (PlayerIndex :type Integer) (Square :type Integer))
  (bind _returnvalue (Math|Integer|%(Integer) Square 40))
  (bind _playerst (Utilities|PlayerbyIndex PlayerIndex))
  (Utilities|Struct|SetmembersinST_Player _playerst _returnvalue)
  (Variables|GamePlay|SetDidLap (<= _returnvalue (Utilities|Struct|BreakST_Player _playerst))))

(fn SetPlayerWallet
  (params (PlayerIndex :type Integer) (Wallet :type Map%20of%20Integers%20to%20Integers))
  (Utilities|Struct|SetmembersinST_Player (Utilities|PlayerbyIndex PlayerIndex) Wallet))

(fn SetPlayerOwnedSquares
  (params (PlayerIndex :type Integer) (Squares :type Array%20of%20BP%20Board%20Square%20Object%20References))
  (Utilities|Struct|SetmembersinST_Player (Utilities|PlayerbyIndex PlayerIndex) Squares))

(fn AddChanceCard
  (params (PlayerIndex :type Integer) (Card :type EN_CHANCE%20Enum :default "NewEnumerator0"))
  (bind _playerst (Utilities|PlayerbyIndex PlayerIndex))
  (bind _chancecards (Utilities|Struct|BreakST_Player _playerst))
  (Utilities|Array|Add _chancecards Card)
  (Utilities|Struct|SetmembersinST_Player _playerst _chancecards))

(fn RemoveChanceCard
  (params (PlayerIndex :type Integer) (Card :type EN_CHANCE%20Enum :default "NewEnumerator0"))
  (bind _playerst (Utilities|PlayerbyIndex PlayerIndex))
  (bind _chancecards (Utilities|Struct|BreakST_Player _playerst))
  (Utilities|Array|RemoveItem _chancecards Card)
  (Utilities|Struct|SetmembersinST_Player _playerst _chancecards))

(fn SetPlayerJailed
  (params (PlayerIndex :type Integer) (Jailed :type Boolean))
  (Utilities|Struct|SetmembersinST_Player (Utilities|PlayerbyIndex PlayerIndex) Jailed))

(fn GetBuildingsCount
  (params (PlayerIndex :type Integer))
  (for _array_element (Utilities|Struct|BreakST_Player (Utilities|PlayerbyIndex PlayerIndex))
    (LocalVariables|SetTotalHouses (+ (Variables|/Game/Monopoly/Blueprints/Board/BP_BoardSquare.BP_BoardSquare_C|GetHousesNumber _array_element) (LocalVariables|GetTotalHouses)))
    (if (Variables|/Game/Monopoly/Blueprints/Board/BP_BoardSquare.BP_BoardSquare_C|GetHasHotel _array_element)
      (Math|Integer|IncrementInt (LocalVariables|GetTotalHotels))))
  (return (LocalVariables|GetTotalHouses) (LocalVariables|GetTotalHotels)))

(fn AddOwnedSquare
  (params (PlayerIndex :type Integer) (Square :type BP%20Board%20Square%20Object%20Reference))
  (bind _playerst (Utilities|PlayerbyIndex PlayerIndex))
  (bind _squares (Utilities|Struct|BreakST_Player _playerst))
  (Default|SetPlayerOwner Square PlayerIndex)
  (Utilities|Array|Add _squares Square)
  (Utilities|Struct|SetmembersinST_Player _playerst _squares))

(fn RemoveOwnedSquare
  (params (PlayerIndex :type Integer) (Square :type BP%20Board%20Square%20Object%20Reference))
  (bind _playerrefs (Variables|References|GetPlayerRefs))
  (bind _output (Utilities|Array|Get(acopy) _playerrefs PlayerIndex))
  (bind _squares (Utilities|Struct|BreakST_Player _output))
  (Default|SetPlayerOwner Square PlayerIndex)
  (Utilities|Array|RemoveItem _squares Square)
  (Utilities|Struct|SetmembersinST_Player _output _squares))

(fn AddCommunityCard
  (params (PlayerIndex :type Integer) (Card :type EN_COMMUNITY%20Enum :default "NewEnumerator0"))
  (bind _playerst (Utilities|PlayerbyIndex PlayerIndex))
  (bind _communitycards (Utilities|Struct|BreakST_Player _playerst))
  (Utilities|Array|Add _communitycards Card)
  (Utilities|Struct|SetmembersinST_Player _playerst _communitycards))

(fn RemoveCommunityCard
  (params (PlayerIndex :type Integer) (Card :type EN_COMMUNITY%20Enum :default "NewEnumerator0"))
  (bind _playerst (Utilities|PlayerbyIndex PlayerIndex))
  (bind _communitycards (Utilities|Struct|BreakST_Player _playerst))
  (Utilities|Array|Add _communitycards Card)
  (Utilities|Struct|SetmembersinST_Player _playerst _communitycards))